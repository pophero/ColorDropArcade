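; BP_Lanterns runs a wave of sprite lanterns that rises or descends through the level, then readies obstacles and balloons after a rise.
; Lanterns_Up picks a random prebuilt row formation sized by league or bonus state, and timelines move it at distance-scaled speed.
; Per-instance colors flicker randomly, while a material Z parameter tracks the cloud layer.
; Idle formations use a disabled material, and the active one is hidden again when movement finishes.
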(event `Lanterns_Down`
  (bind _levellogic (`self.LevelLogic`))
  (bind _lant (`self.Lant`))
  (bind _lant_2 (`self.Lant`))
  (set `self.End_Loc` (`SceneComponent.K2_GetComponentLocation` (`self.Lant`)))
  (`TimelineComponent.SetPlayRate` (`self.Lant_Down_Time`) (/ 5000.0 (`KismetMathLibrary.Abs` (- (.z (`self.Start_Loc`)) (.z (`self.End_Loc`))))))
  (bind (_direction _newtrack_2) (`Timeline|Lant_Down_Time` :!via `PlayFromStart`)
    (:`Update`
      (`SceneComponent.K2_SetWorldLocation` _lant (`KismetMathLibrary.VLerp` (`self.End_Loc`) (`self.Start_Loc`) _newtrack_2) false false)
      (bind _returnvalue (`PrimitiveComponent.CreateDynamicMaterialInstance` (`self.Lant`) 0 "/Game/Materials/Ball_Lant/MI_Sprite_Lant.MI_Sprite_Lant" :!label _label))
      (`MaterialInstanceDynamic.SetScalarParameterValue` _returnvalue "Z" (- (.z (`self.K2_GetActorLocation` (`self.CLOUD_MID`))) 450.0))
      (`SceneComponent.SetHiddenInGame` _lant_2 false false)
      (for _index (range (+ (`PaperGroupedSpriteComponent.GetInstanceCount` _lant_2) 1))
        (bind (_r _g _b) (break `LinearColor` (`|GetArrayItem` (`self.Lant_Color`) _index)))
        (`PaperGroupedSpriteComponent.UpdateInstanceColor` _lant_2 _index (make `LinearColor` _r _g _b (`KismetMathLibrary.RandomFloatInRange` -0.2 0.4)) true))
      (if (> (stale `Lanterns_Up` _newtrack_0) 0.85)
        (`/Engine/EditorBlueprintResources/StandardMacros.DoOnce` false :!label _label_2
          (:`Completed`
            (if (and (>= (`/Game/BluePrints/Level_Logic.Lant_Row_Max` _levellogic) 7) (`KismetMathLibrary.RandomBoolWithWeight` 0.7))
              (`/Game/BluePrints/Level_Logic.Start_Emodji` _levellogic 0))))))
    (:`Finished`
      (`SceneComponent.K2_SetWorldLocation` _lant (0.0 5.0 -1400.0) false false)
      (set `self.Lant_Activate` false :!label _label_3)
      (`SceneComponent.SetHiddenInGame` (`self.Lant`) true false)
      (`self.Set_Lant_Mat` false)
      (goto _label_2 :!via `Reset`))))

(event `Lanterns_Up`
  (bind _my_char (`self.My_Char`))
  (bind _current_lant (`self.Current_Lant`))
  (bind _my_char_2 (`self.My_Char`))
  (bind _levellogic (`self.LevelLogic`))
  (bind _levellogic_2 (`self.LevelLogic`))
  (bind _lant_color (`self.Lant_Color`))
  (bind _linearcolor (make `LinearColor` (`KismetMathLibrary.RandomFloatInRange` 0.33 0.8) (`KismetMathLibrary.RandomFloatInRange` 0.5 1.0) (`KismetMathLibrary.RandomFloatInRange` 0.5 1.0) (`KismetMathLibrary.RandomFloatInRange` -0.1 0.1)))
  (bind _axis_value (`/Game/BluePrints/My_Char.Axis_Value` _my_char))
  (bind _returnvalue (- (`/Game/BluePrints/Level_Logic.Speed_Scale` (`self.LevelLogic`)) 1.0))
  (bind _output_get (set `/Game/BluePrints/Level_Logic.Lant_Row_Max` (select `bool` (and (`/Game/BluePrints/My_Char.Drop_Reverse` _my_char_2) (== (`/Game/BluePrints/Level_Logic.BONUS` _levellogic_2) 4) (`/Game/BluePrints/Level_Logic.Bonus_Activate` _levellogic_2)) :`false` (select `int` (- (`/Game/BluePrints/Level_Logic.League` _levellogic_2) 1) :`0` (`KismetMathLibrary.RandomIntegerInRange` 2 3) :`1` (`KismetMathLibrary.RandomIntegerInRange` 4 6) :`2` (`KismetMathLibrary.RandomIntegerInRange` 7 10)) :`true` (`/Game/BluePrints/My_Char.LL_Lant_Row_Max` _my_char_2)) (`self.LevelLogic`)))
  (set `self.Start_Loc` (0.0 30.0 -1400.0))
  (set `self.End_Loc` (`KismetMathLibrary.MakeVector` 0.0 30.0 (+ -1400.0 (+ (* _output_get 280.0) 2850.0))))
  (set `self.Lant` (select `int` (- (`/Game/BluePrints/Level_Logic.Lant_Row_Max` (`self.LevelLogic`)) 2) :`0` (select `int` (`KismetMathLibrary.RandomIntegerInRange` 0 3) :`0` (`self.Lant_2_Row_00`) :`1` (`self.Lant_2_Row_01`) :`2` (`self.Lant_2_Row_02`) :`3` (`self.Lant_2_Row_03`)) :`1` (select `int` (`KismetMathLibrary.RandomIntegerInRange` 0 2) :`0` (`self.Lant_3_Row_00`) :`1` (`self.Lant_3_Row_01`) :`2` (`self.Lant_3_Row_02`)) :`2` (select `int` (`KismetMathLibrary.RandomIntegerInRange` 0 3) :`0` (`self.Lant_4_Row_00`) :`1` (`self.Lant_4_Row_01`) :`2` (`self.Lant_4_Row_02`) :`3` (`self.Lant_4_Row_03`)) :`3` (select `int` (`KismetMathLibrary.RandomIntegerInRange` 0 3) :`0` (`self.Lant_5_Row_00`) :`1` (`self.Lant_5_Row_01`) :`2` (`self.Lant_5_Row_02`) :`3` (`self.Lant_5_Row_03`)) :`4` (select `int` (`KismetMathLibrary.RandomIntegerInRange` 0 5) :`0` (`self.Lant_6_Row_00`) :`1` (`self.Lant_6_Row_01`) :`2` (`self.Lant_6_Row_02`) :`3` (`self.Lant_6_Row_03`) :`4` (`self.Lant_6_Row_04`) :`5` (`self.Lant_6_Row_05`)) :`5` (select `int` (`KismetMathLibrary.RandomIntegerInRange` 0 5) :`0` (`self.Lant_7_Row_00`) :`1` (`self.Lant_7_Row_01`) :`2` (`self.Lant_7_Row_02`) :`3` (`self.Lant_7_Row_03`) :`4` (`self.Lant_7_Row_04`) :`5` (`self.Lant_7_Row_05`)) :`6` (select `int` (`KismetMathLibrary.RandomIntegerInRange` 0 6) :`0` (`self.Lant_8_Row_00`) :`1` (`self.Lant_8_Row_01`) :`2` (`self.Lant_8_Row_02`) :`3` (`self.Lant_8_Row_03`) :`4` (`self.Lant_8_Row_04`) :`5` (`self.Lant_8_Row_05`) :`6` (`self.Lant_8_Row_06`)) :`7` (select `int` (`KismetMathLibrary.RandomIntegerInRange` 0 7) :`0` (`self.Lant_9_Row_00`) :`1` (`self.Lant_9_Row_01`) :`2` (`self.Lant_9_Row_02`) :`3` (`self.Lant_9_Row_03`) :`4` (`self.Lant_9_Row_04`) :`5` (`self.Lant_9_Row_05`) :`6` (`self.Lant_9_Row_06`) :`7` (`self.Lant_9_Row_07`)) :`8` (select `int` (`KismetMathLibrary.RandomIntegerInRange` 0 7) :`0` (`self.Lant_10_Row_00`) :`1` (`self.Lant_10_Row_01`) :`2` (`self.Lant_10_Row_02`) :`3` (`self.Lant_10_Row_03`) :`4` (`self.Lant_10_Row_04`) :`5` (`self.Lant_10_Row_05`) :`6` (`self.Lant_10_Row_06`) :`7` (`self.Lant_10_Row_07`))))
  (`TimelineComponent.SetPlayRate` (`self.Lant_UP_Time`) (* (select `int` (- (`/Game/BluePrints/Level_Logic.League` (`self.LevelLogic`)) 1) :`0` 0.6 :`1` _returnvalue :`2` _returnvalue) (/ 550.0 (`KismetMathLibrary.Abs` (- (.z (`self.End_Loc`)) (.z (`self.Start_Loc`)))))))
  (set `self.Lant_Activate` true)
  (set `self.Current_Lant` -1)
  (for _index (range (+ (`PaperGroupedSpriteComponent.GetInstanceCount` (`self.Lant`)) 1))
    (`KismetArrayLibrary.Array_Set` _lant_color _index (make `LinearColor` (`KismetMathLibrary.RandomFloatInRange` 0.33 0.8) (`KismetMathLibrary.RandomFloatInRange` 0.5 1.0) (`KismetMathLibrary.RandomFloatInRange` 0.5 1.0) (`KismetMathLibrary.RandomFloatInRange` -0.1 0.1)) true)
    (`PaperGroupedSpriteComponent.UpdateInstanceColor` (`self.Lant`) _index (`|GetArrayItem` _lant_color _index) true))
  (`self.Set_Lant_Mat` true)
  (`|ExecutionSequence`
    (:`then_0`
      (bind (_direction _newtrack_0) (`Timeline|Lant_UP_Time` :!via `PlayFromStart`)
        (:`Update`
          (`SceneComponent.K2_SetWorldLocation` (`self.Lant`) (`KismetMathLibrary.VLerp` (`self.Start_Loc`) (`self.End_Loc`) _newtrack_0) false false)
          (`ParticleSystemComponent.SetFloatParameter` (`/Game/BluePrints/Level_Logic.Lanterns_BG` (`self.LevelLogic`)) "Spawn_Rate" (select `bool` (> _newtrack_0 (select `int` (- (`/Game/BluePrints/Level_Logic.League` (`self.LevelLogic`)) 1) :`0` 0.4 :`1` 0.55 :`2` 0.55 :!type "Float (single-precision)")) :`false` 3.5 :!type "Float (single-precision)"))
          (`Pawn.AddMovementInput` _my_char (0.001 0.0 0.0) (select `bool` (!= _axis_value 0.0) :`false` 0.45 :`true` _axis_value) false)
          (goto _label))
        (:`Finished`
          (set `/Game/BluePrints/Level_Logic.Obstacles_Ready` true _levellogic)
          (`/Game/BluePrints/Level_Logic.Balloones_Spawn` _levellogic)
          (goto _label_3))))
    (:`then_1`
      (set `self.Current_Lant` (`KismetMathLibrary.RandomIntegerInRange` 0 (`PaperGroupedSpriteComponent.GetInstanceCount` (`self.Lant`))) :!label _label_4)
      (`KismetArrayLibrary.Array_Set` (`self.Lant_Color`) _current_lant _linearcolor)
      (`PaperGroupedSpriteComponent.UpdateInstanceColor` (`self.Lant`) _current_lant _linearcolor true)
      (`KismetSystemLibrary.Delay` (`KismetMathLibrary.RandomFloatInRange` 0.1 0.3))
      (if (`self.Lant_Activate`)
        (goto _label_4)))))

(fn `Set_Lant_Mat`
  (params (Start_or_Not :type Boolean))
  (`PrimitiveComponent.SetMaterial` (`self.Lant`) 0 (select `bool` Start_or_Not :`false` "/Game/Materials/Ball_Lant/M_Lant_Disable.M_Lant_Disable" :`true` "/Game/Materials/Ball_Lant/MI_Sprite_Lant.MI_Sprite_Lant" :!type "MaterialInterface Object Reference"))
  (return))

(fn `UserConstructionScript`
  (`PrimitiveComponent.SetMaterial` (`self.Lant_8_Row_00`) 0 (select `bool` false :`false` "/Game/Materials/Ball_Lant/M_Lant_Disable.M_Lant_Disable" :`true` "/Game/Materials/Ball_Lant/M_Sprite_Lant.M_Sprite_Lant" :!type "MaterialInterface Object Reference"))
  (`PrimitiveComponent.SetMaterial` (`self.MAIN`) 0 (select `bool` false :`false` "/Game/Materials/Ball_Lant/M_Lant_Disable.M_Lant_Disable" :`true` "/Game/Materials/Ball_Lant/M_Sprite_Lant.M_Sprite_Lant" :!type "MaterialInterface Object Reference"))
  (`PrimitiveComponent.SetMaterial` (`self.Lant_4_Row_00`) 0 (select `bool` false :`false` "/Game/Materials/Ball_Lant/M_Lant_Disable.M_Lant_Disable" :`true` "/Game/Materials/Ball_Lant/M_Sprite_Lant.M_Sprite_Lant" :!type "MaterialInterface Object Reference"))
  (`PrimitiveComponent.SetMaterial` (`self.Lant_4_Row_01`) 0 (select `bool` false :`false` "/Game/Materials/Ball_Lant/M_Lant_Disable.M_Lant_Disable" :`true` "/Game/Materials/Ball_Lant/M_Sprite_Lant.M_Sprite_Lant" :!type "MaterialInterface Object Reference"))
  (`PrimitiveComponent.SetMaterial` (`self.Lant_4_Row_02`) 0 (select `bool` false :`false` "/Game/Materials/Ball_Lant/M_Lant_Disable.M_Lant_Disable" :`true` "/Game/Materials/Ball_Lant/M_Sprite_Lant.M_Sprite_Lant" :!type "MaterialInterface Object Reference"))
  (`PrimitiveComponent.SetMaterial` (`self.Lant_4_Row_03`) 0 (select `bool` false :`false` "/Game/Materials/Ball_Lant/M_Lant_Disable.M_Lant_Disable" :`true` "/Game/Materials/Ball_Lant/M_Sprite_Lant.M_Sprite_Lant" :!type "MaterialInterface Object Reference"))
  (`PrimitiveComponent.SetMaterial` (`self.Lant_5_Row_00`) 0 (select `bool` false :`false` "/Game/Materials/Ball_Lant/M_Lant_Disable.M_Lant_Disable" :`true` "/Game/Materials/Ball_Lant/M_Sprite_Lant.M_Sprite_Lant" :!type "MaterialInterface Object Reference"))
  (`PrimitiveComponent.SetMaterial` (`self.Lant_5_Row_01`) 0 (select `bool` false :`false` "/Game/Materials/Ball_Lant/M_Lant_Disable.M_Lant_Disable" :`true` "/Game/Materials/Ball_Lant/M_Sprite_Lant.M_Sprite_Lant" :!type "MaterialInterface Object Reference"))
  (`PrimitiveComponent.SetMaterial` (`self.Lant_5_Row_02`) 0 (select `bool` false :`false` "/Game/Materials/Ball_Lant/M_Lant_Disable.M_Lant_Disable" :`true` "/Game/Materials/Ball_Lant/M_Sprite_Lant.M_Sprite_Lant" :!type "MaterialInterface Object Reference"))
  (`PrimitiveComponent.SetMaterial` (`self.Lant_5_Row_03`) 0 (select `bool` false :`false` "/Game/Materials/Ball_Lant/M_Lant_Disable.M_Lant_Disable" :`true` "/Game/Materials/Ball_Lant/M_Sprite_Lant.M_Sprite_Lant" :!type "MaterialInterface Object Reference"))
  (`PrimitiveComponent.SetMaterial` (`self.Lant_6_Row_00`) 0 (select `bool` false :`false` "/Game/Materials/Ball_Lant/M_Lant_Disable.M_Lant_Disable" :`true` "/Game/Materials/Ball_Lant/M_Sprite_Lant.M_Sprite_Lant" :!type "MaterialInterface Object Reference"))
  (`PrimitiveComponent.SetMaterial` (`self.Lant_6_Row_01`) 0 (select `bool` false :`false` "/Game/Materials/Ball_Lant/M_Lant_Disable.M_Lant_Disable" :`true` "/Game/Materials/Ball_Lant/M_Sprite_Lant.M_Sprite_Lant" :!type "MaterialInterface Object Reference"))
  (`PrimitiveComponent.SetMaterial` (`self.Lant_6_Row_02`) 0 (select `bool` false :`false` "/Game/Materials/Ball_Lant/M_Lant_Disable.M_Lant_Disable" :`true` "/Game/Materials/Ball_Lant/M_Sprite_Lant.M_Sprite_Lant" :!type "MaterialInterface Object Reference"))
  (`PrimitiveComponent.SetMaterial` (`self.Lant_6_Row_03`) 0 (select `bool` false :`false` "/Game/Materials/Ball_Lant/M_Lant_Disable.M_Lant_Disable" :`true` "/Game/Materials/Ball_Lant/M_Sprite_Lant.M_Sprite_Lant" :!type "MaterialInterface Object Reference"))
  (`PrimitiveComponent.SetMaterial` (`self.Lant_6_Row_04`) 0 (select `bool` false :`false` "/Game/Materials/Ball_Lant/M_Lant_Disable.M_Lant_Disable" :`true` "/Game/Materials/Ball_Lant/M_Sprite_Lant.M_Sprite_Lant" :!type "MaterialInterface Object Reference"))
  (`PrimitiveComponent.SetMaterial` (`self.Lant_6_Row_05`) 0 (select `bool` false :`false` "/Game/Materials/Ball_Lant/M_Lant_Disable.M_Lant_Disable" :`true` "/Game/Materials/Ball_Lant/M_Sprite_Lant.M_Sprite_Lant" :!type "MaterialInterface Object Reference"))
  (`PrimitiveComponent.SetMaterial` (`self.Lant_7_Row_00`) 0 (select `bool` false :`false` "/Game/Materials/Ball_Lant/M_Lant_Disable.M_Lant_Disable" :`true` "/Game/Materials/Ball_Lant/M_Sprite_Lant.M_Sprite_Lant" :!type "MaterialInterface Object Reference"))
  (`PrimitiveComponent.SetMaterial` (`self.Lant_7_Row_01`) 0 (select `bool` false :`false` "/Game/Materials/Ball_Lant/M_Lant_Disable.M_Lant_Disable" :`true` "/Game/Materials/Ball_Lant/M_Sprite_Lant.M_Sprite_Lant" :!type "MaterialInterface Object Reference"))
  (`PrimitiveComponent.SetMaterial` (`self.Lant_7_Row_02`) 0 (select `bool` false :`false` "/Game/Materials/Ball_Lant/M_Lant_Disable.M_Lant_Disable" :`true` "/Game/Materials/Ball_Lant/M_Sprite_Lant.M_Sprite_Lant" :!type "MaterialInterface Object Reference"))
  (`PrimitiveComponent.SetMaterial` (`self.Lant_7_Row_03`) 0 (select `bool` false :`false` "/Game/Materials/Ball_Lant/M_Lant_Disable.M_Lant_Disable" :`true` "/Game/Materials/Ball_Lant/M_Sprite_Lant.M_Sprite_Lant" :!type "MaterialInterface Object Reference"))
  (`PrimitiveComponent.SetMaterial` (`self.Lant_7_Row_04`) 0 (select `bool` false :`false` "/Game/Materials/Ball_Lant/M_Lant_Disable.M_Lant_Disable" :`true` "/Game/Materials/Ball_Lant/M_Sprite_Lant.M_Sprite_Lant" :!type "MaterialInterface Object Reference"))
  (`PrimitiveComponent.SetMaterial` (`self.Lant_7_Row_05`) 0 (select `bool` false :`false` "/Game/Materials/Ball_Lant/M_Lant_Disable.M_Lant_Disable" :`true` "/Game/Materials/Ball_Lant/M_Sprite_Lant.M_Sprite_Lant" :!type "MaterialInterface Object Reference"))
  (`PrimitiveComponent.SetMaterial` (`self.Lant_10_Row_07`) 0 (select `bool` false :`false` "/Game/Materials/Ball_Lant/M_Lant_Disable.M_Lant_Disable" :`true` "/Game/Materials/Ball_Lant/M_Sprite_Lant.M_Sprite_Lant" :!type "MaterialInterface Object Reference"))
  (`PrimitiveComponent.SetMaterial` (`self.Lant_8_Row_01`) 0 (select `bool` false :`false` "/Game/Materials/Ball_Lant/M_Lant_Disable.M_Lant_Disable" :`true` "/Game/Materials/Ball_Lant/M_Sprite_Lant.M_Sprite_Lant" :!type "MaterialInterface Object Reference"))
  (`PrimitiveComponent.SetMaterial` (`self.Lant_8_Row_02`) 0 (select `bool` false :`false` "/Game/Materials/Ball_Lant/M_Lant_Disable.M_Lant_Disable" :`true` "/Game/Materials/Ball_Lant/M_Sprite_Lant.M_Sprite_Lant" :!type "MaterialInterface Object Reference"))
  (`PrimitiveComponent.SetMaterial` (`self.Lant_8_Row_03`) 0 (select `bool` false :`false` "/Game/Materials/Ball_Lant/M_Lant_Disable.M_Lant_Disable" :`true` "/Game/Materials/Ball_Lant/M_Sprite_Lant.M_Sprite_Lant" :!type "MaterialInterface Object Reference"))
  (`PrimitiveComponent.SetMaterial` (`self.Lant_8_Row_04`) 0 (select `bool` false :`false` "/Game/Materials/Ball_Lant/M_Lant_Disable.M_Lant_Disable" :`true` "/Game/Materials/Ball_Lant/M_Sprite_Lant.M_Sprite_Lant" :!type "MaterialInterface Object Reference"))
  (`PrimitiveComponent.SetMaterial` (`self.Lant_8_Row_05`) 0 (select `bool` false :`false` "/Game/Materials/Ball_Lant/M_Lant_Disable.M_Lant_Disable" :`true` "/Game/Materials/Ball_Lant/M_Sprite_Lant.M_Sprite_Lant" :!type "MaterialInterface Object Reference"))
  (`PrimitiveComponent.SetMaterial` (`self.Lant_8_Row_06`) 0 (select `bool` false :`false` "/Game/Materials/Ball_Lant/M_Lant_Disable.M_Lant_Disable" :`true` "/Game/Materials/Ball_Lant/M_Sprite_Lant.M_Sprite_Lant" :!type "MaterialInterface Object Reference"))
  (`PrimitiveComponent.SetMaterial` (`self.Lant_9_Row_00`) 0 (select `bool` false :`false` "/Game/Materials/Ball_Lant/M_Lant_Disable.M_Lant_Disable" :`true` "/Game/Materials/Ball_Lant/M_Sprite_Lant.M_Sprite_Lant" :!type "MaterialInterface Object Reference"))
  (`PrimitiveComponent.SetMaterial` (`self.Lant_9_Row_01`) 0 (select `bool` false :`false` "/Game/Materials/Ball_Lant/M_Lant_Disable.M_Lant_Disable" :`true` "/Game/Materials/Ball_Lant/M_Sprite_Lant.M_Sprite_Lant" :!type "MaterialInterface Object Reference"))
  (`PrimitiveComponent.SetMaterial` (`self.Lant_9_Row_02`) 0 (select `bool` false :`false` "/Game/Materials/Ball_Lant/M_Lant_Disable.M_Lant_Disable" :`true` "/Game/Materials/Ball_Lant/M_Sprite_Lant.M_Sprite_Lant" :!type "MaterialInterface Object Reference"))
  (`PrimitiveComponent.SetMaterial` (`self.Lant_9_Row_03`) 0 (select `bool` false :`false` "/Game/Materials/Ball_Lant/M_Lant_Disable.M_Lant_Disable" :`true` "/Game/Materials/Ball_Lant/M_Sprite_Lant.M_Sprite_Lant" :!type "MaterialInterface Object Reference"))
  (`PrimitiveComponent.SetMaterial` (`self.Lant_9_Row_04`) 0 (select `bool` false :`false` "/Game/Materials/Ball_Lant/M_Lant_Disable.M_Lant_Disable" :`true` "/Game/Materials/Ball_Lant/M_Sprite_Lant.M_Sprite_Lant" :!type "MaterialInterface Object Reference"))
  (`PrimitiveComponent.SetMaterial` (`self.Lant_9_Row_05`) 0 (select `bool` false :`false` "/Game/Materials/Ball_Lant/M_Lant_Disable.M_Lant_Disable" :`true` "/Game/Materials/Ball_Lant/M_Sprite_Lant.M_Sprite_Lant" :!type "MaterialInterface Object Reference"))
  (`PrimitiveComponent.SetMaterial` (`self.Lant_9_Row_06`) 0 (select `bool` false :`false` "/Game/Materials/Ball_Lant/M_Lant_Disable.M_Lant_Disable" :`true` "/Game/Materials/Ball_Lant/M_Sprite_Lant.M_Sprite_Lant" :!type "MaterialInterface Object Reference"))
  (`PrimitiveComponent.SetMaterial` (`self.Lant_9_Row_07`) 0 (select `bool` false :`false` "/Game/Materials/Ball_Lant/M_Lant_Disable.M_Lant_Disable" :`true` "/Game/Materials/Ball_Lant/M_Sprite_Lant.M_Sprite_Lant" :!type "MaterialInterface Object Reference"))
  (`PrimitiveComponent.SetMaterial` (`self.Lant_10_Row_00`) 0 (select `bool` false :`false` "/Game/Materials/Ball_Lant/M_Lant_Disable.M_Lant_Disable" :`true` "/Game/Materials/Ball_Lant/M_Sprite_Lant.M_Sprite_Lant" :!type "MaterialInterface Object Reference"))
  (`PrimitiveComponent.SetMaterial` (`self.Lant_10_Row_01`) 0 (select `bool` false :`false` "/Game/Materials/Ball_Lant/M_Lant_Disable.M_Lant_Disable" :`true` "/Game/Materials/Ball_Lant/M_Sprite_Lant.M_Sprite_Lant" :!type "MaterialInterface Object Reference"))
  (`PrimitiveComponent.SetMaterial` (`self.Lant_10_Row_02`) 0 (select `bool` false :`false` "/Game/Materials/Ball_Lant/M_Lant_Disable.M_Lant_Disable" :`true` "/Game/Materials/Ball_Lant/M_Sprite_Lant.M_Sprite_Lant" :!type "MaterialInterface Object Reference"))
  (`PrimitiveComponent.SetMaterial` (`self.Lant_10_Row_03`) 0 (select `bool` false :`false` "/Game/Materials/Ball_Lant/M_Lant_Disable.M_Lant_Disable" :`true` "/Game/Materials/Ball_Lant/M_Sprite_Lant.M_Sprite_Lant" :!type "MaterialInterface Object Reference"))
  (`PrimitiveComponent.SetMaterial` (`self.Lant_10_Row_04`) 0 (select `bool` false :`false` "/Game/Materials/Ball_Lant/M_Lant_Disable.M_Lant_Disable" :`true` "/Game/Materials/Ball_Lant/M_Sprite_Lant.M_Sprite_Lant" :!type "MaterialInterface Object Reference"))
  (`PrimitiveComponent.SetMaterial` (`self.Lant_10_Row_05`) 0 (select `bool` false :`false` "/Game/Materials/Ball_Lant/M_Lant_Disable.M_Lant_Disable" :`true` "/Game/Materials/Ball_Lant/M_Sprite_Lant.M_Sprite_Lant" :!type "MaterialInterface Object Reference"))
  (`PrimitiveComponent.SetMaterial` (`self.Lant_10_Row_06`) 0 (select `bool` false :`false` "/Game/Materials/Ball_Lant/M_Lant_Disable.M_Lant_Disable" :`true` "/Game/Materials/Ball_Lant/M_Sprite_Lant.M_Sprite_Lant" :!type "MaterialInterface Object Reference"))
  (`PrimitiveComponent.SetMaterial` (`self.Lant_2_Row_00`) 0 (select `bool` false :`false` "/Game/Materials/Ball_Lant/M_Lant_Disable.M_Lant_Disable" :`true` "/Game/Materials/Ball_Lant/M_Sprite_Lant.M_Sprite_Lant" :!type "MaterialInterface Object Reference"))
  (`PrimitiveComponent.SetMaterial` (`self.Lant_2_Row_01`) 0 (select `bool` false :`false` "/Game/Materials/Ball_Lant/M_Lant_Disable.M_Lant_Disable" :`true` "/Game/Materials/Ball_Lant/M_Sprite_Lant.M_Sprite_Lant" :!type "MaterialInterface Object Reference"))
  (`PrimitiveComponent.SetMaterial` (`self.Lant_2_Row_02`) 0 (select `bool` false :`false` "/Game/Materials/Ball_Lant/M_Lant_Disable.M_Lant_Disable" :`true` "/Game/Materials/Ball_Lant/M_Sprite_Lant.M_Sprite_Lant" :!type "MaterialInterface Object Reference"))
  (`PrimitiveComponent.SetMaterial` (`self.Lant_2_Row_03`) 0 (select `bool` false :`false` "/Game/Materials/Ball_Lant/M_Lant_Disable.M_Lant_Disable" :`true` "/Game/Materials/Ball_Lant/M_Sprite_Lant.M_Sprite_Lant" :!type "MaterialInterface Object Reference"))
  (`PrimitiveComponent.SetMaterial` (`self.Lant_3_Row_00`) 0 (select `bool` false :`false` "/Game/Materials/Ball_Lant/M_Lant_Disable.M_Lant_Disable" :`true` "/Game/Materials/Ball_Lant/M_Sprite_Lant.M_Sprite_Lant" :!type "MaterialInterface Object Reference"))
  (`PrimitiveComponent.SetMaterial` (`self.Lant_3_Row_01`) 0 (select `bool` false :`false` "/Game/Materials/Ball_Lant/M_Lant_Disable.M_Lant_Disable" :`true` "/Game/Materials/Ball_Lant/M_Sprite_Lant.M_Sprite_Lant" :!type "MaterialInterface Object Reference"))
  (`PrimitiveComponent.SetMaterial` (`self.Lant_3_Row_02`) 0 (select `bool` false :`false` "/Game/Materials/Ball_Lant/M_Lant_Disable.M_Lant_Disable" :`true` "/Game/Materials/Ball_Lant/M_Sprite_Lant.M_Sprite_Lant" :!type "MaterialInterface Object Reference")))