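; BP_Buble_Gift is a touchable gift bubble that floats up the screen and pops for a running score.
; Bubble_Start randomizes position by Index band, labeling the first two bubbles "TOUCH" and "US" as a prompt.
; A timeline lerps it upward with sideways wobble, its play rate scaled by distance for steady speed.
; When LevelLogic allows, touch hides the bubble, plays a burst sound and shows the incremented BubbleGiftCounter.
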(event `Bubble_Start`
  (bind _bubble_gift (`self.Bubble_Gift`))
  (bind _index (`self.Index`))
  (bind _touch (`self.Touch`))
  (bind _index_2 (`self.Index`))
  (bind _returnvalue (`KismetMathLibrary.Conv_IntToDouble` (`KismetMathLibrary.RandomIntegerInRange` 0 200)))
  (bind _returnvalue_2 (`KismetMathLibrary.Conv_IntToDouble` (`KismetMathLibrary.RandomIntegerInRange` 200 450)))
  (bind _y (.y (`self.Start_Loc`)))
  (bind _returnvalue_3 (`KismetMathLibrary.Conv_IntToDouble` (`KismetMathLibrary.RandomIntegerInRange` -450 -200)))
  (bind _returnvalue_4 (`KismetMathLibrary.Conv_IntToDouble` (`KismetMathLibrary.RandomIntegerInRange` -200)))
  (`|ExecutionSequence`
    (:`then_0`
      (`SceneComponent.K2_SetWorldLocation` _bubble_gift (`KismetMathLibrary.MakeVector` (select `int` (`self.Index`) :`0` (`KismetMathLibrary.Conv_IntToDouble` (`KismetMathLibrary.RandomIntegerInRange` -200 -100)) :`1` (`KismetMathLibrary.Conv_IntToDouble` (`KismetMathLibrary.RandomIntegerInRange` 100 200)) :`2` _returnvalue_3 :`3` _returnvalue_3 :`4` _returnvalue_3 :`5` _returnvalue_4 :`6` _returnvalue_4 :`7` _returnvalue_4 :`8` _returnvalue :`9` _returnvalue :`10` _returnvalue :`11` _returnvalue_2 :`12` _returnvalue_2 :`13` _returnvalue_2 :`14` _returnvalue_2) 215.0 (`KismetMathLibrary.Conv_IntToDouble` (select `bool` (< _index 2) :`false` (`KismetMathLibrary.RandomIntegerInRange` -2600 -1600) :`true` (select `int` _index :`0` -1450 :`1` -1350)))) false false)
      (bind _output_get (set `self.Start_Loc` (`SceneComponent.K2_GetComponentLocation` _bubble_gift)))
      (set `self.End_Loc` (`KismetMathLibrary.MakeVector` (.x _output_get) (.y _output_get) 1450.0))
      (`TimelineComponent.SetPlayRate` (`self.Timeline_0`) (/ (select `bool` (< (`self.Index`) 2) :`false` 450.0 :`true` 475.0 :!type "Float (single-precision)") (- (.z (`self.End_Loc`)) (.z (`self.Start_Loc`)))))
      (bind (_direction _up _side) (`Timeline|Timeline_0` :!via `PlayFromStart`)
        (:`Update`
          (bind _returnvalue_5 (+ (`KismetMathLibrary.Lerp` 0.0 (select `bool` (`self.Bubble_End`) :`false` 25.0 :!type "Float (single-precision)") _side) (.x (`self.Start_Loc`))))
          (`SceneComponent.K2_SetWorldLocation` (`self.Bubble_Gift`) (`KismetMathLibrary.VLerp` (`KismetMathLibrary.MakeVector` _returnvalue_5 _y (.z (`self.Start_Loc`))) (`KismetMathLibrary.MakeVector` _returnvalue_5 _y 1450.0) _up) false false))
        (:`Finished`
          (set `self.Bubble_End` true))))
    (:`then_1`
      (if (< (`self.Index`) 2)
        (`SceneComponent.SetHiddenInGame` (`self.Touch`) false false)
        (if (== _index_2 0)
          (`TextRenderComponent.K2_SetText` _touch "TOUCH")
          (`TextRenderComponent.SetWorldSize` _touch 30.0)
          (elif (== _index_2 1)
            (`TextRenderComponent.K2_SetText` _touch "US")
            (`TextRenderComponent.SetWorldSize` _touch 40.0)))))))

(event `self.Bubble_Gift.OnInputTouchBegin`
  (params (FingerIndex :type "ETouchIndex Enum" :default "Touch1") (TouchedComponent :type "PrimitiveComponent Object Reference"))
  (bind _bubble_gift (`self.Bubble_Gift`))
  (bind _count (`self.Count`))
  (bind _levellogic (`self.LevelLogic`))
  (if (and (`/Game/BluePrints/Level_Logic.Can_Bubble_Gift` _levellogic) (`/Game/BluePrints/Level_Logic.Input` _levellogic))
    (if (not (`self.Bubble_End`))
      (`SceneComponent.SetHiddenInGame` _bubble_gift true false)
      (`SceneComponent.SetHiddenInGame` (`self.Touch`) true false)
      (`PaperSpriteComponent.SetSprite` _bubble_gift "/Game/Sprites/Bubble/SP_Bubble_Gift_End.SP_Bubble_Gift_End")
      (`PrimitiveComponent.SetCollisionEnabled` _bubble_gift "NoCollision")
      (`SceneComponent.SetHiddenInGame` _count false false)
      (bind _result (`/Engine/EditorBlueprintResources/StandardMacros.IncrementInt` (`/Game/BluePrints/Level_Logic.Bubble_Gift_Counter` (`self.LevelLogic`)))
        (:`  `
          (`TextRenderComponent.K2_SetText` _count (`KismetTextLibrary.Conv_IntToText` _result))
          (set `self.Bubble_End` true)
          (`GameplayStatics.PlaySound2D` "/Game/Sounds/Bubble_Burst.Bubble_Burst"))))))

(fn `UserConstructionScript`)