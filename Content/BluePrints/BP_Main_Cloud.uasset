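; Sprite-based cloud, in a middle or right variant, that reports player overlap begin and end to LevelLogic.
; Set_Cloud randomizes eight front/back puff pairs, tints them from LevelLogic's random index, stores drift endpoints for MovePart's lerp and starts eight timelines.
; On the middle cloud, one index triggers delayed lightning sprite flashes with storm particles, and another activates magic particles.
; The construction script previews the layout using the Color setting.
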(event `self.MAIN_CLOUD.OnComponentBeginOverlap`
  (params (OverlappedComponent :type "PrimitiveComponent Object Reference") (OtherActor :type "Actor Object Reference") (OtherComp :type "PrimitiveComponent Object Reference") (OtherBodyIndex :type Integer) (bFromSweep :type Boolean) (SweepResult :type "HitResult Structure (by ref)"))
  (bind _levellogic (`self.LevelLogic`))
  (cast `/Game/BluePrints/My_Char` OtherActor)
  (if (`self.Right_Cloud`)
    (`/Game/BluePrints/Level_Logic.CLOUD_RIGHT_OVERLAP` _levellogic)
    (else
      (`/Game/BluePrints/Level_Logic.CLOUD_MID_OVERLAP` _levellogic))))

(event `self.CLOUD_Overlap.OnComponentEndOverlap`
  (params (OverlappedComponent :type "PrimitiveComponent Object Reference") (OtherActor :type "Actor Object Reference") (OtherComp :type "PrimitiveComponent Object Reference") (OtherBodyIndex :type Integer))
  (cast `/Game/BluePrints/My_Char` OtherActor)
  (`/Game/BluePrints/Level_Logic.CLOUD_END_OVERLAP` (`self.LevelLogic`)))

(event `Set_Cloud`
  (bind _right_cloud (`self.Right_Cloud`))
  (bind _storm_part (`self.Storm_Part`))
  (bind _storm_part_2 (`self.Storm_Part`))
  (bind _levellogic (`self.LevelLogic`))
  (bind _returnvalue (select `int` (`KismetMathLibrary.RandomIntegerInRange` 0 2) :`0` 0.85 :`1` 0.925 :`2` 1.0 :!type "Float (single-precision)"))
  (bind _returnvalue_2 (select `bool` (`self.Right_Cloud`) :`false` (`/Game/BluePrints/Level_Logic.Cloud_Random` _levellogic) :`true` (`/Game/BluePrints/Level_Logic.Cloud_Random1` _levellogic)))
  (`SceneComponent.SetVisibility` (`self.Lightning_Cloud_Part_08`) false false)
  (`SceneComponent.SetVisibility` (`self.Lightning_Cloud_Part_09`) false false)
  (`SceneComponent.SetVisibility` (`self.Lightning_Cloud_Part_10`) false false)
  (`SceneComponent.SetVisibility` (`self.Lightning_Cloud_Part_Back_08`) false false)
  (`SceneComponent.SetVisibility` (`self.Lightning_Cloud_Part_Back_09`) false false)
  (`SceneComponent.SetVisibility` (`self.Lightning_Cloud_Part_Back_10`) false false)
  (`ActorComponent.Deactivate` (`self.Storm_Part`))
  (for (_array_element _array_index) (`|MakeArray` (`self.Cloud_Part_00`) (`self.Cloud_Part_01`) (`self.Cloud_Part_02`) (`self.Cloud_Part_03`) (`self.Cloud_Part_04`) (`self.Cloud_Part_05`) (`self.Cloud_Part_06`) (`self.Cloud_Part_07`))
    (`SceneComponent.K2_SetRelativeLocation` _array_element (`KismetMathLibrary.MakeVector` (+ (.x (`|GetArrayItem` (`self.Cloud_Part_Loc_Array_NEW`) _array_index)) (`KismetMathLibrary.Conv_IntToDouble` (`KismetMathLibrary.RandomIntegerInRange` -50 50)) (select `bool` (`self.Right_Cloud`) :`true` 829.0 :!type "Float (single-precision)")) (.y (`|GetArrayItem` (`self.Cloud_Part_Loc_Array_NEW`) _array_index)) (+ (.z (`|GetArrayItem` (`self.Cloud_Part_Loc_Array_NEW`) _array_index)) (`KismetMathLibrary.Conv_IntToDouble` (`KismetMathLibrary.RandomIntegerInRange` -70 70)))) false false)
    (`SceneComponent.SetRelativeScale3D` _array_element (`KismetMathLibrary.MakeVector` _returnvalue 1.0 _returnvalue))
    (set `self.Current_Sprite_Index` (`KismetMathLibrary.RandomIntegerInRange` 0 3))
    (`PaperSpriteComponent.SetSprite` (`self.MAIN_CLOUD`) (select `bool` _right_cloud :`false` "/Game/Sprites/Clouds/SP_C_Mid_Forw.SP_C_Mid_Forw" :`true` "/Game/Sprites/Clouds/SP_C_Right_Forw.SP_C_Right_Forw" :!type "PaperSprite Object Reference"))
    (`PaperSpriteComponent.SetSprite` (`self.MAIN_CLOUD_Back`) (select `bool` _right_cloud :`false` "/Game/Sprites/Clouds/SP_C_Mid_Back.SP_C_Mid_Back" :`true` "/Game/Sprites/Clouds/SP_C_Right_Back.SP_C_Right_Back" :!type "PaperSprite Object Reference"))
    (`PaperSpriteComponent.SetSpriteColor` (`self.MAIN_CLOUD`) (`|GetArrayItem` (`self.Cloud_Colors`) _returnvalue_2))
    (`PaperSpriteComponent.SetSpriteColor` (`self.MAIN_CLOUD_Back`) (`|GetArrayItem` (`self.Cloud_Colors`) _returnvalue_2))
    (`PaperSpriteComponent.SetSprite` _array_element (`|GetArrayItem` (`self.Sprite_Array_Forw`) (`self.Current_Sprite_Index`)))
    (`PaperSpriteComponent.SetSprite` (`|GetArrayItem` (`|MakeArray` (`self.Cloud_Part_Back_00`) (`self.Cloud_Part_Back_01`) (`self.Cloud_Part_Back_02`) (`self.Cloud_Part_Back_03`) (`self.Cloud_Part_Back_04`) (`self.Cloud_Part_Back_05`) (`self.Cloud_Part_Back_06`) (`self.Cloud_Part_Back_07`)) _array_index) (`|GetArrayItem` (`self.Sprite_Array_Back`) (`self.Current_Sprite_Index`)))
    (`PaperSpriteComponent.SetSpriteColor` _array_element (`|GetArrayItem` (`self.Cloud_Colors`) _returnvalue_2))
    (`PaperSpriteComponent.SetSpriteColor` (`|GetArrayItem` (`|MakeArray` (`self.Cloud_Part_Back_00`) (`self.Cloud_Part_Back_01`) (`self.Cloud_Part_Back_02`) (`self.Cloud_Part_Back_03`) (`self.Cloud_Part_Back_04`) (`self.Cloud_Part_Back_05`) (`self.Cloud_Part_Back_06`) (`self.Cloud_Part_Back_07`)) _array_index) (`|GetArrayItem` (`self.Cloud_Colors`) _returnvalue_2))
    (bind _relativelocation (`SceneComponent.RelativeLocation` _array_element))
    (`KismetArrayLibrary.Array_Set` (`self.C_Part_Start_Loc`) _array_index _relativelocation true)
    (`KismetArrayLibrary.Array_Set` (`self.C_Part_End_Loc`) _array_index (`KismetMathLibrary.MakeVector` (+ (.x _relativelocation) (`KismetMathLibrary.Conv_IntToDouble` (select `bool` (`self.Right_Cloud`) :`false` (`KismetMathLibrary.RandomIntegerInRange` -150 -20) :`true` (`KismetMathLibrary.RandomIntegerInRange` 20 150)))) (.y _relativelocation) (.z _relativelocation)) true))
  (`PaperSpriteComponent.SetSprite` (`self.CLOUD_Overlap`) (select `bool` (`self.Right_Cloud`) :`false` "/Game/Sprites/Clouds/SP_C_Overlap_Mid.SP_C_Overlap_Mid" :`true` "/Game/Sprites/Clouds/SP_C_Overlap_Right.SP_C_Overlap_Right" :!type "PaperSprite Object Reference"))
  (`TimelineComponent.PlayFromStart` (`self.Timeline_0`))
  (`TimelineComponent.PlayFromStart` (`self.Timeline_1`))
  (`TimelineComponent.PlayFromStart` (`self.Timeline_2`))
  (`TimelineComponent.PlayFromStart` (`self.Timeline_3`))
  (`TimelineComponent.PlayFromStart` (`self.Timeline_4`))
  (`TimelineComponent.PlayFromStart` (`self.Timeline_5`))
  (`TimelineComponent.PlayFromStart` (`self.Timeline_6`))
  (`TimelineComponent.PlayFromStart` (`self.Timeline_7`))
  (if (and (== (`/Game/BluePrints/Level_Logic.Cloud_Random` (`self.LevelLogic`)) 7) (== (`self.Right_Cloud`) false))
    (`KismetSystemLibrary.Delay` (`KismetMathLibrary.RandomFloatInRange` 0.7 1.2))
    (`SceneComponent.SetVisibility` (`self.Lightning_Cloud_Part_08`) (`KismetMathLibrary.RandomBool`) false)
    (`SceneComponent.SetVisibility` (`self.Lightning_Cloud_Part_Back_08`) (`KismetMathLibrary.RandomBool`) false)
    (`SceneComponent.SetVisibility` (`self.Lightning_Cloud_Part_Back_09`) (`KismetMathLibrary.RandomBool`) false)
    (`SceneComponent.SetVisibility` (`self.Lightning_Cloud_Part_09`) (`KismetMathLibrary.RandomBool`) false)
    (`SceneComponent.SetVisibility` (`self.Lightning_Cloud_Part_10`) (`KismetMathLibrary.RandomBool`) false)
    (`SceneComponent.SetVisibility` (`self.Lightning_Cloud_Part_Back_10`) (`KismetMathLibrary.RandomBool`) false)
    (`self.Storm_Part_Macro1`
      (:`Out`
        (`|ExecutionSequence`
          (:`then_0`
            (`KismetSystemLibrary.Delay` 0.15)
            (`SceneComponent.SetVisibility` (`self.Lightning_Cloud_Part_08`) false false)
            (`SceneComponent.SetVisibility` (`self.Lightning_Cloud_Part_09`) false false)
            (`SceneComponent.SetVisibility` (`self.Lightning_Cloud_Part_10`) false false)
            (`SceneComponent.SetVisibility` (`self.Lightning_Cloud_Part_Back_08`) false false)
            (`SceneComponent.SetVisibility` (`self.Lightning_Cloud_Part_Back_09`) false false)
            (`SceneComponent.SetVisibility` (`self.Lightning_Cloud_Part_Back_10`) false false)
            (`KismetSystemLibrary.Delay` (`KismetMathLibrary.RandomFloatInRange` 0.7 1.2))
            (`SceneComponent.SetVisibility` (`self.Lightning_Cloud_Part_08`) (`KismetMathLibrary.RandomBool`) false)
            (`SceneComponent.SetVisibility` (`self.Lightning_Cloud_Part_Back_08`) (`KismetMathLibrary.RandomBool`) false)
            (`SceneComponent.SetVisibility` (`self.Lightning_Cloud_Part_Back_09`) (`KismetMathLibrary.RandomBool`) false)
            (`SceneComponent.SetVisibility` (`self.Lightning_Cloud_Part_09`) (`KismetMathLibrary.RandomBool`) false)
            (`SceneComponent.SetVisibility` (`self.Lightning_Cloud_Part_10`) (`KismetMathLibrary.RandomBool`) false)
            (`SceneComponent.SetVisibility` (`self.Lightning_Cloud_Part_Back_10`) (`KismetMathLibrary.RandomBool`) false)
            (`ActorComponent.Activate` _storm_part true)
            (`self.Storm_Part_Macro1`
              (:`Out`
                (`KismetSystemLibrary.Delay` 0.15)
                (`SceneComponent.SetVisibility` (`self.Lightning_Cloud_Part_08`) false false)
                (`SceneComponent.SetVisibility` (`self.Lightning_Cloud_Part_09`) false false)
                (`SceneComponent.SetVisibility` (`self.Lightning_Cloud_Part_10`) false false)
                (`SceneComponent.SetVisibility` (`self.Lightning_Cloud_Part_Back_08`) false false)
                (`SceneComponent.SetVisibility` (`self.Lightning_Cloud_Part_Back_09`) false false)
                (`SceneComponent.SetVisibility` (`self.Lightning_Cloud_Part_Back_10`) false false)
                (`KismetSystemLibrary.Delay` 0.3)
                (`ActorComponent.Deactivate` _storm_part))))
          (:`then_1`
            (`ActorComponent.Activate` _storm_part_2 true)
            (`KismetSystemLibrary.Delay` 0.3)
            (`ActorComponent.Deactivate` _storm_part_2)))))
    (else
      (`ActorComponent.SetActive` (`self.Magic_Part`) (and (== (`/Game/BluePrints/Level_Logic.Cloud_Random` (`self.LevelLogic`)) 8) (== (`self.Right_Cloud`) false)) true))))

(fn `Move_Part`
  (params (Target :type "PaperSpriteComponent Object Reference") (Alpha :type "Float (double-precision)"))
  (bind _returnvalue (`KismetArrayLibrary.Array_Find` (`|MakeArray` (`self.Cloud_Part_00`) (`self.Cloud_Part_01`) (`self.Cloud_Part_02`) (`self.Cloud_Part_03`) (`self.Cloud_Part_04`) (`self.Cloud_Part_05`) (`self.Cloud_Part_06`) (`self.Cloud_Part_07`)) Target))
  (`SceneComponent.K2_SetRelativeLocation` Target (`KismetMathLibrary.VLerp` (`|GetArrayItem` (`self.C_Part_Start_Loc`) _returnvalue) (`|GetArrayItem` (`self.C_Part_End_Loc`) _returnvalue) Alpha) false false))

(fn `UserConstructionScript`
  (bind _right_cloud (`self.Right_Cloud`))
  (`SceneComponent.SetVisibility` (`self.Lightning_Cloud_Part_08`) false false)
  (`SceneComponent.SetVisibility` (`self.Lightning_Cloud_Part_09`) false false)
  (`SceneComponent.SetVisibility` (`self.Lightning_Cloud_Part_10`) false false)
  (`SceneComponent.SetVisibility` (`self.Lightning_Cloud_Part_Back_08`) false false)
  (`SceneComponent.SetVisibility` (`self.Lightning_Cloud_Part_Back_09`) false false)
  (`SceneComponent.SetVisibility` (`self.Lightning_Cloud_Part_Back_10`) false false)
  (for (_array_element _array_index) (`|MakeArray` (`self.Cloud_Part_00`) (`self.Cloud_Part_01`) (`self.Cloud_Part_02`) (`self.Cloud_Part_03`) (`self.Cloud_Part_04`) (`self.Cloud_Part_05`) (`self.Cloud_Part_06`) (`self.Cloud_Part_07`))
    (`SceneComponent.K2_SetRelativeLocation` _array_element (`KismetMathLibrary.MakeVector` (+ (.x (`|GetArrayItem` (`self.Cloud_Part_Loc_Array_NEW`) _array_index)) (select `bool` (`self.Right_Cloud`) :`true` 829.0 :!type "Float (single-precision)")) (.y (`|GetArrayItem` (`self.Cloud_Part_Loc_Array_NEW`) _array_index)) (.z (`|GetArrayItem` (`self.Cloud_Part_Loc_Array_NEW`) _array_index))) false false)
    (set `self.Current_Sprite_Index` (`KismetMathLibrary.RandomIntegerInRange` 0 3))
    (`PaperSpriteComponent.SetSprite` _array_element (`|GetArrayItem` (`self.Sprite_Array_Forw`) (`self.Current_Sprite_Index`)))
    (`PaperSpriteComponent.SetSprite` (`|GetArrayItem` (`|MakeArray` (`self.Cloud_Part_Back_00`) (`self.Cloud_Part_Back_01`) (`self.Cloud_Part_Back_02`) (`self.Cloud_Part_Back_03`) (`self.Cloud_Part_Back_04`) (`self.Cloud_Part_Back_05`) (`self.Cloud_Part_Back_06`) (`self.Cloud_Part_Back_07`)) _array_index) (`|GetArrayItem` (`self.Sprite_Array_Back`) (`self.Current_Sprite_Index`)))
    (`PaperSpriteComponent.SetSpriteColor` _array_element (`|GetArrayItem` (`self.Cloud_Colors`) (`self.Color`)))
    (`PaperSpriteComponent.SetSpriteColor` (`|GetArrayItem` (`|MakeArray` (`self.Cloud_Part_Back_00`) (`self.Cloud_Part_Back_01`) (`self.Cloud_Part_Back_02`) (`self.Cloud_Part_Back_03`) (`self.Cloud_Part_Back_04`) (`self.Cloud_Part_Back_05`) (`self.Cloud_Part_Back_06`) (`self.Cloud_Part_Back_07`)) _array_index) (`|GetArrayItem` (`self.Cloud_Colors`) (`self.Color`))))
  (`PaperSpriteComponent.SetSprite` (`self.MAIN_CLOUD`) (select `bool` _right_cloud :`false` "/Game/Sprites/Clouds/SP_C_Mid_Forw.SP_C_Mid_Forw" :`true` "/Game/Sprites/Clouds/SP_C_Right_Forw.SP_C_Right_Forw" :!type "PaperSprite Object Reference"))
  (`PaperSpriteComponent.SetSprite` (`self.MAIN_CLOUD_Back`) (select `bool` _right_cloud :`false` "/Game/Sprites/Clouds/SP_C_Mid_Back.SP_C_Mid_Back" :`true` "/Game/Sprites/Clouds/SP_C_Right_Back.SP_C_Right_Back" :!type "PaperSprite Object Reference"))
  (`PaperSpriteComponent.SetSpriteColor` (`self.MAIN_CLOUD`) (`|GetArrayItem` (`self.Cloud_Colors`) (`self.Color`)))
  (`PaperSpriteComponent.SetSpriteColor` (`self.MAIN_CLOUD_Back`) (`|GetArrayItem` (`self.Cloud_Colors`) (`self.Color`)))
  (`PaperSpriteComponent.SetSprite` (`self.CLOUD_Overlap`) (select `bool` (`self.Right_Cloud`) :`false` "/Game/Sprites/Clouds/SP_C_Overlap_Mid.SP_C_Overlap_Mid" :`true` "/Game/Sprites/Clouds/SP_C_Overlap_Right.SP_C_Overlap_Right" :!type "PaperSprite Object Reference")))